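; Measurement tool actor that spawns a BP_Dimenssion between surface points picked with the mouse cursor.
; Measure deprojects the cursor into a visibility line trace and, on a hit, spawns the dimension with both endpoints there.
; A looping timer then repeats the trace to move PointB to the surface under the cursor, with no stop logic here.
; Both traces draw persistent debug lines.
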(event Custom|Measure
  (bind _returnvalue (Game|GetPlayerController 0))
  (bind (_worldlocation _worlddirection) (Game|Player|ConvertMouseLocationToWorldSpace _returnvalue))
  (bind (_outhit _returnvalue_2) (Collision|LineTraceByChannel _worldlocation (+ _worldlocation (* _worlddirection 1e+04)) "TraceTypeQuery1" true 0 "Persistent"))
  (if _returnvalue_2
    (bind _returnvalue_3 (Game|SpawnActorfromClass "/MeasureDistance/MeasureDistanceTool/Blueprints/Commands/Dimension/BPs/BP_Dimenssion.BP_Dimenssion_C" (Math|Transform|MakeTransform "0, 0, 0" "0, 0, 0" "1,1,1") "Undefined" 0 (.Location (Collision|BreakHitResult _outhit)) (.Location (Collision|BreakHitResult _outhit)) 0 "NewEnumerator1" false 0))
    (Variables|Default|SetMeasureActor _returnvalue_3)
    (Utilities|Time|SetTimerbyEvent (delegate Custom|GetPointB_Event) 0.3 true)))

(event Custom|GetPointB_Event
  (bind _returnvalue (Game|GetPlayerController 0))
  (bind (_worldlocation _worlddirection) (Game|Player|ConvertMouseLocationToWorldSpace _returnvalue))
  (bind (_outhit _returnvalue_2) (Collision|LineTraceByChannel _worldlocation (+ _worldlocation (* _worlddirection 1e+04)) "TraceTypeQuery1" true 0 "Persistent"))
  (if _returnvalue_2
    (Variables|/MeasureDistance/MeasureDistanceTool/Blueprints/Commands/Dimension/BPs/BP_Dimenssion.BP_Dimenssion_C|SetPointB (Variables|Default|GetMeasureActor) (.Location (Collision|BreakHitResult _outhit)))))

(fn ConstructionScript)