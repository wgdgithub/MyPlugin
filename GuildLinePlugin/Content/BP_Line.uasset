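; BP_Line is a spline-based Blueprint that draws a visible guide line out of repeated static meshes.
; Its SpawnGuidLine event adds a caller-specified number of mesh components at even distances along the spline, matching its local position and rotation.
; Each mesh is lowered by the supplied capsule half-height, takes the given mesh and scale, and has collision disabled.
; The construction script is empty, so meshes appear only when the event is called.
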(event Custom|SpawnGuidLine
  (params (LineAccount :type Integer) (LineDistance :type Float%20%28single-precision%29) (LineMeshRelativeTransformScale :type Vector) (LineStaticMesh :type Static%20Mesh%20Object%20Reference) (CapsuleHalfHeight :type Float%20%28single-precision%29))
  (bind _spline (Variables|Default|GetSpline))
  (for _index (range 0 (- LineAccount 1))
    (bind _returnvalue (AddComponent|AddStaticMeshComponent false (Math|Transform|MakeTransform (Math|Vector|MakeVector (.x (Spline|GetLocationatDistanceAlongSpline _spline (* _index LineDistance) "Local")) (.y (Spline|GetLocationatDistanceAlongSpline _spline (* _index LineDistance) "Local")) (- (.z (Spline|GetLocationatDistanceAlongSpline _spline (* _index LineDistance) "Local")) CapsuleHalfHeight)) (Spline|GetRotationatDistanceAlongSpline _spline (* _index LineDistance) "Local") LineMeshRelativeTransformScale)))
    (Components|StaticMesh|SetStaticMesh _returnvalue LineStaticMesh)
    (Collision|SetCollisionEnabled _returnvalue "NoCollision")
    (Development|SetHiddeninGame _returnvalue false false)))

(fn ConstructionScript)